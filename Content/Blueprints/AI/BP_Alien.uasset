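; BP_Alien is a spider-like enemy character that chases the player and plays a melee attack animation up close.
; A BeginPlay AI MoveTo loop re-issues the chase after a short delay until death.
; Tick checks distance to the BP_Marine player, pauses movement for the attack montage and restores it on completion.
; Incoming damage lowers Health; at zero it sets Death, stopping new attacks and disabling capsule and mesh collision.
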(event EventBeginPlay
  (if (Variables|Default|Getdeath) :!label _label
    (Development|PrintString "umarłem")
    (else
      (AI|AIMoveTo self "0, 0, 0" (Game|GetPlayerCharacter 0) 5.0 false
        (:OnSuccess
          _)
        (:OnFail
          _))
      (Utilities|FlowControl|Delay 0.2)
      (goto _label))))

(event Game|Damage|EventAnyDamage
  (params (Damage :type Float%20%28single-precision%29) (DamageType :type Damage%20Type%20Object%20Reference) (InstigatedBy :type Controller%20Object%20Reference) (DamageCauser :type Actor%20Object%20Reference))
  (CallFunction|AppleDamage Damage))

(event EventTick
  (params (DeltaSeconds :type Float%20%28single-precision%29))
  (if (not (Variables|Default|Getdeath))
    (if (and (CallFunction|IsAttackRange) (not (CallFunction|IsAttacking)))
      (CallFunction|NewFunction0)
      (Animation|Montage|PlayMontage (Variables|Character|GetMesh) "/Game/Characters/Enemy_Great_Spider/Animations/spiderattack.spiderattack" 1.5
        (:OnCompleted
          (CallFunction|SpiderMovmentActive))))))

(fn ConstructionScript)

(fn IsAttackRange
  (bind _asbp_marine (Utilities|Casting|CastToBP_Marine (Game|Player|GetPlayerPawn 0)))
  (return (< (Transformation|GetDistanceTo _asbp_marine) 1e+02)))

(fn IsAttacking
  (return (Animation|Montage|MontageIsPlaying (Components|SkeletalMesh|GetAnimInstance (Variables|Character|GetMesh)) "/Game/Characters/Enemy_Great_Spider/Animations/spiderattack.spiderattack")))

(fn SpiderMovmentActive
  (if (not (Variables|Default|Getdeath))
    (Components|Activation|Activate (Variables|Character|GetCharacterMovement) false)))

(fn NewFunction0
  (Components|Activation|Deactivate (Variables|Character|GetCharacterMovement)))

(fn AppleDamage
  (params (damage :type Float%20%28single-precision%29))
  (bind _output_get (Variables|Default|SetHealth (- (Variables|Default|GetHealth) damage)))
  (if (== (Math|Float|Clamp(Float) _output_get 0.0 1e+02) 0.0)
    (bind _output_get_2 (Variables|Default|Setdeath true))
    (Collision|SetCollisionEnabled (Variables|Collision|GetCapsuleComponent) "NoCollision")
    (return (not _output_get_2))))